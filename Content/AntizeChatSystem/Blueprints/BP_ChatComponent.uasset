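; Player controller chat component that links the local chat and player list widgets to the server.
; On local BeginPlay it requests a PlayerID from the GameMode via interface, retrying before creating the widgets.
; The server routes messages by category (all, global, proximity, private, team, system) by scanning PlayerControllers and relaying through each one's component via client RPC.
; It also handles team changes, online checks for private messages, blocking and local combat logs.
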(event Custom|Server_GetPlayerIsOnline
  (params (ToPlayerID :type Integer) (ToUsername :type Text))
  ;[1 1 1] Check if the PlayerID is online (Server->Client)
  (bind _online_ (PrivateMessage|OnServerGetPlayerIsOnline ToPlayerID))
  (CallFunction|ClientGetPlayerIsOnline _online_ ToPlayerID ToUsername))

(event Custom|Client_GetPlayerIsOnline
  (params (PlayerOnline? :type Boolean) (ToPlayerID :type Integer) (ToUsername :type Text))
  (bind _mainchatref (Variables|Spawn|GetMainChatRef))
  ;[1 1 1] Check if the PlayerID is online (Server->Client)
  (if PlayerOnline?
    (Default|ContinueonClickedPrivateMessage _mainchatref ToPlayerID ToUsername)
    (else
      (Default|PlayerNotFound _mainchatref ToUsername))))

(event Custom|Server_RequestSendPrivateMessage
  (params (ByCommand? :type Boolean) (ToPlayerID :type Integer) (ToUsername :type Text) (Message :type Text) (FromUsername :type Text))
  ;[1 1 1] Check if the Player is online and send the message (Server->Client)
  (PrivateMessage|OnRequestSendPrivateMessage ByCommand? ToPlayerID ToUsername Message FromUsername))

(event Custom|Client_RequestSendPrivateMessage
  (params (PlayerOnline? :type Boolean) (ToPlayerID :type Integer) (ToUsername :type Text) (Message :type Text) (FromUsername :type Text))
  (bind _mainchatref (Variables|Spawn|GetMainChatRef))
  ;[1 1 1] Check if the Player is online and send the message (Server->Client)
  (if PlayerOnline?
    (Default|ContinuePrivateMessage _mainchatref ToPlayerID ToUsername Message FromUsername)
    (else
      (Default|PlayerNotFound _mainchatref ToUsername))))

(event Custom|Server_RequestPlayerID
  ;[1 1 1] Set player ID (Server)
  (Utilities|MyHasAuthority
    (:Server
      (bind (_playerid _success_) (Class|BPChatInterface|MSGChatRequestPlayerID(Message) (Game|GetGameMode)))
      (if _success_
        (Variables|Spawn|SetPlayerID _playerid)))))

(event Custom|Server_SendMessage
  (params (OwnControler :type Controller%20Object%20Reference) (MessageDate :type S%20Message%20Data%20Structure))
  ;[1 1 1] Received or Send a Message (Server|Client)
  ;;[1 1 1] Send Message to Players (Server)
  (Utilities|MyHasAuthority
    (:Server
      (Traitement|OnServerSendMessage (Variables|Traitement|GetTeamID) OwnControler MessageDate))))

(event Custom|Client_RefreshTeam
  (params (TeamID :type Integer))
  (bind _playerlisrref (Variables|Spawn|GetPlayerLisrRef))
  (bind _mainchatref (Variables|Spawn|GetMainChatRef))
  ;[1 1 1] Set Team ID (Server->Client)
  (Utilities|IsValid _mainchatref
    (:Is%20Valid
      (Default|ShowTeamMessage _mainchatref TeamID))
    (:Is%20Not%20Valid
      _))
  (Utilities|IsValid _playerlisrref
    (:Is%20Valid
      (Utilities|FlowControl|Delay 0.2)
      (Default|RefreshActualTeam _playerlisrref))))

(event Custom|Client_ReceivedMessage
  (params (MessageData :type S%20Message%20Data%20Structure%20%28by%20ref%29))
  (bind _mainchatref (Variables|Spawn|GetMainChatRef))
  ;[1 1 1] Received or Send a Message (Server|Client)
  ;;[1 1 1] Received Message (OwningClient)
  (Utilities|IsValid _mainchatref
    (:Is%20Valid
      (Default|ReceivedMessage _mainchatref MessageData true))))

(event Custom|Server_SetTeamID
  (params (TeamID :type Integer))
  ;[1 1 1] Set Team ID (Server->Client)
  (Utilities|MyHasAuthority
    (:Server
      (if (!= (Variables|Traitement|GetTeamID) TeamID)
        (bind _output_get (Variables|Traitement|SetTeamID TeamID))
        (CallFunction|ClientRefreshTeam _output_get)))))

(event Custom|CallSetBlockedPlayer
  (params (Blocked? :type Boolean) (Username :type Text))
  (bind _mainchatref (Variables|Spawn|GetMainChatRef))
  ;[1 1 1] Block/Unblock player (Client)
  (Utilities|IsValid _mainchatref
    (:Is%20Valid
      (Default|SetBlockedPlayer _mainchatref Blocked? Username))))

(event Custom|OnNewMessage
  (params (Received? :type Boolean) (MessageData :type S%20Message%20Data%20Structure))
  ;[1 1 1] Received or Send a Message (Server|Client)
  (if Received?
    (CallFunction|ClientReceivedMessage MessageData)
    (else
      (CallFunction|ServerSendMessage (Variables|Spawn|GetControllerRef) MessageData))))

(event EventBeginPlay
  ;[1 1 1] Constructeur Create MainChat Widget (Delay, be sure to have PlayerID)
  ;;[1 1 1] Only on local player
  (Utilities|OnLocalPlayer
    (:true
      (CallFunction|ServerRequestPlayerID)
      ;;[1 1 1] Wait for the PlayerID
      (if (>= (Variables|Spawn|GetPlayerID) 0) :!label _label
        _
        (else
          (bind _result (Math|Integer|IncrementInt (Variables|Spawn|GetAttempt))
            (:%20%20
              (if (>= _result 600)
                (Development|PrintString "Unable to obtain a PlayerID, check if you have implemented MSG_RequestPlayerID in the GameMode and \"Success?\" is checked." true true "(R=1.000000,G=0.000000,B=0.007345,A=1.000000)" 25.0)
                (else
                  (Utilities|FlowControl|Delay 0.1)
                  (goto _label)))))))
      (bind _returnvalue (UserInterface|CreateWidget "/Game/AntizeChatSystem/Widgets/W_MainChat.W_MainChat_C" 0 (Variables|Spawn|GetPlayerID) (Variables|Spawn|GetControllerRef) self))
      (bind _output_get (Variables|Spawn|SetMainChatRef _returnvalue))
      (UserInterface|Viewport|AddtoViewport _output_get 1)
      (bind _returnvalue_2 (UserInterface|CreateWidget "/Game/AntizeChatSystem/Widgets/W_PlayerList.W_PlayerList_C" 0 self))
      (bind _output_get_2 (Variables|Spawn|SetPlayerLisrRef _returnvalue_2))
      (UserInterface|Viewport|AddtoViewport _output_get_2 2))))

(fn OpenChat
  (bind _mainchatref (Variables|Spawn|GetMainChatRef))
  (bind _playerlisrref (Variables|Spawn|GetPlayerLisrRef))
  (Utilities|IsValid _playerlisrref
    (:Is%20Valid
      (if (Variables|/Game/AntizeChatSystem/Widgets/W_PlayerList.W_PlayerList_C|GetIsVisible? _playerlisrref)
        (return)
        (else
          _)))
    (:Is%20Not%20Valid
      _))
  (Utilities|IsValid _mainchatref
    (:Is%20Valid
      (Default|OpenCloseChat _mainchatref)
      (return))
    (:Is%20Not%20Valid
      (return))))

(fn OpenPlayerList
  (bind _playerlisrref (Variables|Spawn|GetPlayerLisrRef))
  (Utilities|IsValid _playerlisrref
    (:Is%20Valid
      (Default|ShowHide _playerlisrref false)
      (return))
    (:Is%20Not%20Valid
      (return))))

(fn OnServerGetPlayerIsOnline
  (params (ToPlayerID :type Integer))
  (Utilities|MyHasAuthority
    (:Server
      (if (>= ToPlayerID 0)
        (bind _outactors (Actor|GetAllActorsOfClass "/Script/Engine.PlayerController"))
        (bind _array_element (Utilities|Array|ForEachLoopwithBreak _outactors :!label _label)
          (:LoopBody
            (Utilities|IsValid _array_element
              (:Is%20Valid
                (Utilities|IsValid (Actor|GetComponentbyClass _array_element "BP_ChatComponent_C")
                  (:Is%20Valid
                    (if (== ToPlayerID (Variables|BP_ChatComponent_C|GetPlayerID (Actor|GetComponentbyClass _array_element "BP_ChatComponent_C")))
                      (LocalVariables|SetLocal_Online? true)
                      (goto _label Break)))))))
          (:Completed
            (return (LocalVariables|GetLocal_Online?))))
        (else
          (return false))))
    (:Remote
      (return false))))

(fn OnServerGetPlayerIDfromUsername
  (params (Username :type Text%20%28by%20ref%29))
  (Utilities|MyHasAuthority
    (:Server
      (bind _outactors (Actor|GetAllActorsOfClass "/Script/Engine.PlayerController"))
      (bind _array_element (Utilities|Array|ForEachLoopwithBreak _outactors :!label _label)
        (:LoopBody
          (Utilities|IsValid _array_element
            (:Is%20Valid
              (bind (_success_ _username) (Class|BPChatInterface|MSGChatGetUsername(Message) _array_element))
              (if _success_
                (if (Utilities|Enum|Equal(Enum) (Class|KismetTextLibrary|TexttoUpper _username) (Class|KismetTextLibrary|TexttoUpper Username))
                  (Utilities|IsValid (Actor|GetComponentbyClass _array_element "BP_ChatComponent_C")
                    (:Is%20Valid
                      (LocalVariables|SetLocal_PlayerID (Variables|BP_ChatComponent_C|GetPlayerID (Actor|GetComponentbyClass _array_element "BP_ChatComponent_C")))
                      (goto _label Break))))))))
        (:Completed
          (return (LocalVariables|GetLocal_PlayerID)))))
    (:Remote
      (return (LocalVariables|GetLocal_PlayerID)))))

(fn OnRequestSendPrivateMessage
  (params (ByCommand? :type Boolean) (ToPlayerID :type Integer) (ToUsername :type Text) (Message :type Text) (FromUsername :type Text))
  (if ByCommand?
    (bind _playerid (PrivateMessage|OnServerGetPlayerIDfromUsername ToUsername))
    (bind _output_get (LocalVariables|SetLocal_ToPlayerID _playerid))
    (LocalVariables|SetLocal_IsOnline? (>= _output_get 0))
    (else
      (bind _output_get_2 (LocalVariables|SetLocal_ToPlayerID ToPlayerID))
      (bind _online_ (PrivateMessage|OnServerGetPlayerIsOnline _output_get_2))
      (LocalVariables|SetLocal_IsOnline? _online_)))
  (CallFunction|ClientRequestSendPrivateMessage (LocalVariables|GetLocal_IsOnline?) (LocalVariables|GetLocal_ToPlayerID) ToUsername Message FromUsername)
  (return))

(fn GetIsBlocked
  (params (Username :type Text))
  (bind _mainchatref (Variables|Spawn|GetMainChatRef))
  (Utilities|IsValid _mainchatref
    (:Is%20Valid
      (bind _blocked_ (Default|CheckBlocked _mainchatref Username))
      (return _blocked_))
    (:Is%20Not%20Valid
      (return false))))

(fn OnRepPlayerID
  (bind _controllerref (Variables|Spawn|GetControllerRef))
  (Utilities|IsValid _controllerref
    (:Is%20Valid
      (if (Pawn|IsLocalController _controllerref)
        (Utilities|IsValid (Variables|Spawn|GetMainChatRef)
          (:Is%20Valid
            (Variables|/Game/AntizeChatSystem/Widgets/W_MainChat.W_MainChat_C|SetPlayerID (Variables|Spawn|GetMainChatRef) (Variables|Spawn|GetPlayerID))
            (return))
          (:Is%20Not%20Valid
            _))))
    (:Is%20Not%20Valid
      _))
  (return))

(fn OnServerSendMessage
  (params (OwnTeamID :type Integer) (OwnController :type Controller%20Object%20Reference) (MessageData :type S%20Message%20Data%20Structure))
  (LocalVariables|SetLocal_OwnTeamID OwnTeamID)
  (LocalVariables|SetLocal_OwnController OwnController)
  (LocalVariables|SetLocal_MessageData MessageData)
  (if (and (Utilities|Enum|Equal(Enum) (Utilities|Struct|BreakS_MessageData (LocalVariables|GetLocal_MessageData)) "NewEnumerator6") (<= (LocalVariables|GetLocal_OwnTeamID) -1))
    (return)
    (else
      (bind _outactors (Actor|GetAllActorsOfClass "/Script/Engine.PlayerController"))
      (bind _array_element (Utilities|Array|ForEachLoopwithBreak _outactors :!label _label)
        (:LoopBody
          (bind _output_get (LocalVariables|SetLocal_PlayerController _array_element))
          (Utilities|IsValid _output_get
            (:Is%20Valid
              (switch Utilities|FlowControl|Switch|SwitchonE_ChatCategory (Utilities|Struct|BreakS_MessageData (LocalVariables|GetLocal_MessageData))
                (:NewEnumerator3
                  (CallFunction|OnNewMessage (Actor|GetComponentbyClass (LocalVariables|GetLocal_PlayerController) "BP_ChatComponent_C") true (LocalVariables|GetLocal_MessageData) :!label _label_2))
                (:NewEnumerator0
                  (goto _label_2))
                (:NewEnumerator1
                  (Utilities|IsValid (Pawn|GetControlledPawn (LocalVariables|GetLocal_OwnController))
                    (:Is%20Valid
                      (Utilities|IsValid (Pawn|GetControlledPawn (LocalVariables|GetLocal_PlayerController))
                        (:Is%20Valid
                          (if (<= (Math|Vector|VectorLength (- (Transformation|GetActorLocation (Pawn|GetControlledPawn (LocalVariables|GetLocal_OwnController))) (Transformation|GetActorLocation (Pawn|GetControlledPawn (LocalVariables|GetLocal_PlayerController))))) (Variables|Settings|GetMaxProximityDistance))
                            (goto _label_2)))))))
                (:NewEnumerator4
                  (Utilities|IsValid (Actor|GetComponentbyClass (LocalVariables|GetLocal_PlayerController) "BP_ChatComponent_C")
                    (:Is%20Valid
                      (if (== (Variables|BP_ChatComponent_C|GetPlayerID (Actor|GetComponentbyClass (LocalVariables|GetLocal_PlayerController) "BP_ChatComponent_C")) (Utilities|Struct|BreakS_MessageData (LocalVariables|GetLocal_MessageData)))
                        (CallFunction|OnNewMessage (Actor|GetComponentbyClass (LocalVariables|GetLocal_PlayerController) "BP_ChatComponent_C") true (LocalVariables|GetLocal_MessageData))
                        (goto _label Break)))))
                (:NewEnumerator5
                  (goto _label_2))
                (:NewEnumerator6
                  (Utilities|IsValid (Actor|GetComponentbyClass (LocalVariables|GetLocal_PlayerController) "BP_ChatComponent_C")
                    (:Is%20Valid
                      (if (== (Variables|BP_ChatComponent_C|GetTeamID (Actor|GetComponentbyClass (LocalVariables|GetLocal_PlayerController) "BP_ChatComponent_C")) (LocalVariables|GetLocal_OwnTeamID))
                        (goto _label_2)))))))))
        (:Completed
          (return))))))

(fn AddCombatLog
  (params (Message :type Text))
  (Default|ReceivedMessage (Variables|Spawn|GetMainChatRef) (Utilities|Struct|MakeS_MessageData "NewEnumerator7" -1 -1 Message) false)
  (return))