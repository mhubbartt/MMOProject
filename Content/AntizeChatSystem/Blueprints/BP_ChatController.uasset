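; BP_ChatController is a controller for the Antize chat system that connects player input and the possessed pawn to a chat component.
; On BeginPlay it registers itself with BPChatComponent, and the Enter and P keys open the chat and player list.
; Chat interface functions return player and team IDs from the component, while username lookups and emotes forward to the controlled pawn.
; The player ID request is a stub that always reports failure.
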(event EventBeginPlay
  ;[1 0 0] Make sure the BeginPlay is implemented in your controller
  (|CallParentFunction)
  (Variables|/Game/AntizeChatSystem/Blueprints/BP_ChatComponent.BP_ChatComponent_C|SetControllerRef (Variables|Default|GetBP_ChatComponent) self))

(event EventMSGChatPlayEmote
  (params (EmoteToPlay :type E_Emote%20Enum :default "NewEnumerator0"))
  (bind _returnvalue (Pawn|GetControlledPawn))
  ;[1 1 1] Play emote
  (Utilities|IsValid _returnvalue
    (:Is%20Valid
      (Class|BPChatInterface|MSGChatPlayEmote(Message) _returnvalue EmoteToPlay))))

(event Input|KeyboardEvents|Enter
  (params (Key :type Key%20Structure))
  ;[1 1 1] Open Close Chat and player list
  (:Pressed
    (Default|OpenChat (Variables|Default|GetBP_ChatComponent))))

(event Input|KeyboardEvents|P
  (params (Key :type Key%20Structure))
  ;[1 1 1] Open Close Chat and player list
  (:Pressed
    (Default|OpenPlayerList (Variables|Default|GetBP_ChatComponent))))

(fn ConstructionScript)

(fn MSGChatGetPlayerID
  (return (Variables|/Game/AntizeChatSystem/Blueprints/BP_ChatComponent.BP_ChatComponent_C|GetPlayerID (Variables|Default|GetBP_ChatComponent))))

(fn MSGChatGetTeamID
  (return (Variables|/Game/AntizeChatSystem/Blueprints/BP_ChatComponent.BP_ChatComponent_C|GetTeamID (Variables|Default|GetBP_ChatComponent))))

(fn MSGChatGetUsername
  (bind _returnvalue (Pawn|GetControlledPawn))
  (Utilities|IsValid _returnvalue
    (:Is%20Valid
      (bind (_success_ _username) (Class|BPChatInterface|MSGChatGetUsername(Message) _returnvalue))
      (return _success_ _username))
    (:Is%20Not%20Valid
      (return false "No pawn found (You must try again)"))))

(fn MSGChatRequestPlayerID
  (return 0 false))