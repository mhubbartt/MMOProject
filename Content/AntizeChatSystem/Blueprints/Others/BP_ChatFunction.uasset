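; Shared helper functions for the Antize chat system, covering timestamps, system messages and player IDs.
; GetActualTime formats the current clock time as an hours:minutes text.
; OnServerSendSystemMessageToPlayers loops over all PlayerControllers and passes a message with no sender or target ID to each BP_ChatComponent as received.
; GetNewPlayerID issues player IDs by incrementing the integer counter passed to it.
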(fn GetActualTime
  (bind _returnvalue (Math|DateTime|Now))
  (bind _returnvalue_2 (TimeOfDay|GetTimeOfDay _returnvalue :!class /Script/Engine.KismetMathLibrary))
  (return (Utilities|Text|FormatText "{HH}:{MM}" (Utilities|Text|ToText(Integer) (.hours _returnvalue_2) false true 2 2) (Utilities|Text|ToText(Integer) (.minutes _returnvalue_2) false true 2 2))))

(fn OnServerSendSystemMessagetoPlayers
  (params (Message :type Text))
  ;[1 1 1] Sends a system message to players
  (bind _outactors (Actor|GetAllActorsOfClass 0 "/Script/Engine.PlayerController"))
  (for _array_element _outactors
    (Utilities|IsValid _array_element
      (:Is%20Valid
        (Default|OnNewMessage (Actor|GetComponentbyClass _array_element "/Game/AntizeChatSystem/Blueprints/BP_ChatComponent.BP_ChatComponent_C") true (Utilities|Struct|MakeS_MessageData "NewEnumerator5" -1 -1 Message)))))
  (return))

(fn GetNewPlayerID
  (params (ActualPlayerID :type Integer%20%28by%20ref%29))
  ;[1 1 1] Get a new PlayerID and increment the given integer variable
  (LocalVariables|SetLocal_PlayerID ActualPlayerID)
  (bind _result (Math|Integer|IncrementInt ActualPlayerID)
    (:%20%20
      (return _result))))